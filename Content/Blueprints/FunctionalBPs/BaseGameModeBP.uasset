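; Game mode Blueprint that creates the player's character HUD and starts a hard-coded introductory quest on BeginPlay.
; It constructs a BaseQuest object, fills in its details and objectives, and keeps references to both quest and HUD.
; The quest's name and description feed the HUD's quest panel, and each objective gets its own ObjectiveInfo widget in a vertical box.
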(event `self.ReceiveBeginPlay`
  (bind _questinfo (`/Game/Blueprints/Widgets/CharacterHUD.QuestInfo` (`self.HUDReference`)))
  (bind _returnvalue (`|CreateWidget` "/Game/Blueprints/Widgets/CharacterHUD.CharacterHUD_C" (`GameplayStatics.GetPlayerController` 0)))
  (bind _output_get (set `self.HUDReference` _returnvalue))
  (`UserWidget.AddToViewport` _output_get 0)
  (bind _returnvalue_2 (`|GenericCreateObject` self "/Script/FirstRPG.BaseQuest"))
  (bind _output_get_2 (set `self.Current Quest Reference` _returnvalue_2))
  (`BaseQuest.SetNumObjectives` _output_get_2 2)
  (`BaseQuest.SetQuestDetails` _output_get_2 "Getting Started" "Basics of first quest")
  (`BaseQuest.SetUpObjective` _output_get_2 0 null null "Slay 1 Witch" 1)
  (`BaseQuest.SetUpObjective` _output_get_2 1 null null "Collect 2 Pickups" 2)
  (`/Game/Blueprints/Widgets/QuestInfo.SetQuestNameText` _questinfo (`KismetTextLibrary.Conv_StringToText` (`BaseQuest.name` _output_get_2)))
  (`/Game/Blueprints/Widgets/QuestInfo.SetQuestDescriptionText` _questinfo (`KismetTextLibrary.Conv_StringToText` (`BaseQuest.description` _output_get_2)))
  (`Widget.SetVisibility` _questinfo "SelfHitTestInvisible")
  (for _array_element (`BaseQuest.objectives` (`self.Current Quest Reference`))
    (bind _returnvalue_3 (`|CreateWidget` "/Game/Blueprints/Widgets/ObjectiveInfo.ObjectiveInfo_C"))
    (`/Game/Blueprints/Widgets/ObjectiveInfo.SetObjectiveDescriptionText` _returnvalue_3 (`KismetTextLibrary.Conv_StringToText` (`.description` (break `Objective` _array_element))))
    (`VerticalBox.AddChildToVerticalBox` (`/Game/Blueprints/Widgets/CharacterHUD.ObjectiveVerticalBox` (`self.HUDReference`)) _returnvalue_3)))

(fn `UserConstructionScript`)