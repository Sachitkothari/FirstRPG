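; Base weapon actor for an RPG that the character can equip and remove, with SetCorrectItemName left empty, apparently for child weapons to override.
; Overlapping its InteractionBox flags FirstRPGCharacter and shows an EquipItemPrompt widget, cleared on exit.
; AttachWeapon destroys any current weapon, attaches its mesh to WeaponSocket and scales attack speed from base speed and dexterity.
; RemoveWeapon destroys the equipped weapon and resets attack speed.
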(event `RemoveWeapon`
  (params (CharacterReference :type "FirstRPGCharacter Object Reference"))
  (bind _currentweapon (`FirstRPGCharacter.currentWeapon` CharacterReference)
    (:`then`
      (bind _asbase_weapon_bp (cast `/Game/Blueprints/Objects/Weapons/BaseWeaponBP` _currentweapon))
      (bind _weaponmesh (`/Game/Blueprints/Objects/Weapons/BaseWeaponBP.WeaponMesh` _asbase_weapon_bp))
      (`PrimitiveComponent.SetCollisionEnabled` _weaponmesh "NoCollision")
      (`SceneComponent.K2_DetachFromComponent` _weaponmesh "KeepRelative" "KeepRelative" "KeepRelative" true)
      (set `FirstRPGCharacter.attackSpeed` 1.0 CharacterReference)
      (`self.K2_DestroyActor` _currentweapon))
    (:`else`)))

(event `AttachWeapon`
  (params (CharacterReference :type "FirstRPGCharacter Object Reference"))
  (bind _currentweapon (`FirstRPGCharacter.currentWeapon` CharacterReference)
    (:`then`
      (bind _asbase_weapon_bp (cast `/Game/Blueprints/Objects/Weapons/BaseWeaponBP` _currentweapon))
      (bind _weaponmesh (`/Game/Blueprints/Objects/Weapons/BaseWeaponBP.WeaponMesh` _asbase_weapon_bp))
      (`PrimitiveComponent.SetCollisionEnabled` _weaponmesh "NoCollision")
      (`SceneComponent.K2_DetachFromComponent` _weaponmesh "KeepRelative" "KeepRelative" "KeepRelative" true)
      (`self.K2_DestroyActor` _currentweapon))
    (:`else`
      _))
  (bind _output_get (set `FirstRPGCharacter.currentWeapon` self CharacterReference))
  (`SceneComponent.K2_AttachToComponent` (`self.WeaponMesh`) (`Character.Mesh` CharacterReference) "WeaponSocket" "KeepRelative" "KeepRelative" "KeepRelative" true)
  (set `FirstRPGCharacter.attackSpeed` (* (`DefaultWeapon.baseSpeed` _output_get) (`FirstRPGCharacter.dexterityValue` CharacterReference)) CharacterReference))

(event `self.InteractionBox.OnComponentBeginOverlap`
  (params (OverlappedComponent :type "PrimitiveComponent Object Reference") (OtherActor :type "Actor Object Reference") (OtherComp :type "PrimitiveComponent Object Reference") (OtherBodyIndex :type Integer) (bFromSweep :type Boolean) (SweepResult :type "HitResult Structure (by ref)"))
  (bind _asfirst_rpgcharacter (cast `FirstRPGCharacter` OtherActor))
  (set `FirstRPGCharacter.isOverlappingItem` true _asfirst_rpgcharacter)
  (bind _returnvalue (`|CreateWidget` "/Game/Blueprints/Widgets/EquipItemPrompt.EquipItemPrompt_C"))
  (`self.SetCorrectItemName` _returnvalue)
  (`UserWidget.AddToViewport` _returnvalue 0))

(event `self.InteractionBox.OnComponentEndOverlap`
  (params (OverlappedComponent :type "PrimitiveComponent Object Reference") (OtherActor :type "Actor Object Reference") (OtherComp :type "PrimitiveComponent Object Reference") (OtherBodyIndex :type Integer))
  (bind _asfirst_rpgcharacter (cast `FirstRPGCharacter` OtherActor))
  (set `FirstRPGCharacter.isOverlappingItem` false _asfirst_rpgcharacter)
  (bind _foundwidgets (`WidgetBlueprintLibrary.GetAllWidgetsOfClass` "/Game/Blueprints/Widgets/EquipItemPrompt.EquipItemPrompt_C"))
  (for _array_element _foundwidgets
    (`Widget.RemoveFromParent` _array_element)))

(fn `SetCorrectItemName`
  (params (WidgetReference :type "/Game/Blueprints/Widgets/EquipItemPrompt Object Reference")))

(fn `UserConstructionScript`)